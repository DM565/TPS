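; EnemyGun_BP is an enemy weapon actor that hands itself to an AIEnemy_BP in the level.
; On BeginPlay it finds one via GetActorOfClass and calls its pickup-weapon function (拾取武器) with itself.
; It repeats the lookup and pickup every three seconds, destroying itself when the found enemy is dead.
; The construction script writes a self reference into the GunInform struct, keeping the other fields.
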(event EventTick
  (params (DeltaSeconds :type Float%20%28single-precision%29)))

(event EventBeginPlay
  (bind _returnvalue (Actor|GetActorOfClass "/Game/TPS_File/AI/AIEnemy_BP.AIEnemy_BP_C" :!label _label))
  (Default|拾取武器 _returnvalue self)
  (if (Variables|/Game/TPS_File/AI/AIEnemy_BP.AIEnemy_BP_C|Getisdead _returnvalue)
    (Actor|DestroyActor)
    (else
      (Utilities|FlowControl|Delay 3.0)
      (goto _label))))

(fn ConstructionScript
  (Variables|Default|SetGun_Inform (Utilities|Struct|MakeGun_Inform_2 (.gun_type (Variables|Default|GetGun_Inform)) self (.图标 (Variables|Default|GetGun_Inform)) (.名称 (Variables|Default|GetGun_Inform)) (.速度 (Variables|Default|GetGun_Inform)) (.声音 (Variables|Default|GetGun_Inform)) (.弹夹容量 (Variables|Default|GetGun_Inform)) (.当前装弹量 (Variables|Default|GetGun_Inform)) (.伤害值 (Variables|Default|GetGun_Inform)) (.gunholdsocket (Variables|Default|GetGun_Inform)) (.gunequipsocket (Variables|Default|GetGun_Inform)) (.shootmontage (Variables|Default|GetGun_Inform)))))