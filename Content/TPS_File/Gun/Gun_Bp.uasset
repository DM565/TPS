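; Gun_Bp is a weapon pickup actor that the player character can collect by pressing F.
; A Sphere overlap caches the Charactor_Bp, sets a pickup flag and enables player 0 input on the gun; leaving the sphere clears both cached values.
; Pressing F passes the gun to the character's 拾取武器 (pick up weapon) function.
; The construction script stamps the actor's own class into its GunInform weapon data struct.
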(event OnComponentBeginOverlap(Sphere)
  (params (OverlappedComponent :type Primitive%20Component%20Object%20Reference) (OtherActor :type Actor%20Object%20Reference) (OtherComp :type Primitive%20Component%20Object%20Reference) (OtherBodyIndex :type Integer) (bFromSweep :type Boolean) (SweepResult :type Hit%20Result%20Structure%20%28by%20ref%29))
  (bind _ascharactor_bp (Utilities|Casting|CastToCharactor_Bp OtherActor))
  (Variables|Default|SetAs%20Charactor%20Bp _ascharactor_bp)
  (Variables|Default|Setpickup？ true)
  (Input|EnableInput (Game|GetPlayerController 0)))

(event OnComponentEndOverlap(Sphere)
  (params (OverlappedComponent :type Primitive%20Component%20Object%20Reference) (OtherActor :type Actor%20Object%20Reference) (OtherComp :type Primitive%20Component%20Object%20Reference) (OtherBodyIndex :type Integer))
  (Variables|Default|SetAs%20Charactor%20Bp 0)
  (Variables|Default|Setpickup？ false))

(event EventBeginPlay)

(event Collision|EventActorBeginOverlap
  (params (OtherActor :type Actor%20Object%20Reference)))

(event EventTick
  (params (DeltaSeconds :type Float%20%28single-precision%29)))

(event Input|KeyboardEvents|F
  (params (Key :type Key%20Structure :default "None"))
  (bind _as_charactor_bp (Variables|Default|GetAs%20Charactor%20Bp))
  (:Pressed
    (Utilities|IsValid _as_charactor_bp
      (:Is%20Valid
        (if (Variables|Default|Getpickup？)
          (Default|拾取武器 _as_charactor_bp self))))))

(fn ConstructionScript
  (Variables|Default|SetGun_Inform (Utilities|Struct|MakeGun_Inform (.gun_type (Variables|Default|GetGun_Inform)) (Utilities|GetClass self) (.图标 (Variables|Default|GetGun_Inform)) (.名称 (Variables|Default|GetGun_Inform)) (.速度 (Variables|Default|GetGun_Inform)) (.声音 (Variables|Default|GetGun_Inform)) (.弹夹容量 (Variables|Default|GetGun_Inform)) (.当前装弹量 (Variables|Default|GetGun_Inform)) (.伤害值 (Variables|Default|GetGun_Inform)) (.gunholdsocket (Variables|Default|GetGun_Inform)) (.gunequipsocket (Variables|Default|GetGun_Inform)) (.shootmontage (Variables|Default|GetGun_Inform)))))