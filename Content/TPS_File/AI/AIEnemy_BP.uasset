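; AI enemy character for a third-person shooter that can hold a gun, take damage and die.
; The construction script assigns AI_Controllor, and the 拾取武器 event snaps a gun onto the mesh at the socket named in its GunInform.
; Harm lowers Health and refreshes the AI_UI widget's health bar; at zero it flags death, stops movement and destroys the actor after a delay.
; AIShoot is an empty stub.
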(event Custom|拾取武器
  (params (Gun :type Enemy%20Gun%20BP%20Object%20Reference))
  (Utilities|IsValid Gun
    (:Is%20Valid
      (Transformation|AttachComponentToComponent Gun (Variables|Character|GetMesh) (.Gunequipsocket (Utilities|Struct|BreakGun_Inform_2 (Variables|/Game/TPS_File/Gun/EnemyGun_BP.EnemyGun_BP_C|GetGun_Inform Gun))) "SnapToTarget" "SnapToTarget" "SnapToTarget" true))))

(event EventBeginPlay
  (Variables|Default|SetHealth (Variables|Default|GetMaxHealth))
  (CallFunction|UpdataUI))

(event EventTick
  (params (DeltaSeconds :type Float%20%28single-precision%29)))

(event EventHarm
  (params (harm :type Float%20%28single-precision%29) (玩家是否死亡 :type Boolean))
  (bind _output_get (Variables|Default|SetHealth (- (Variables|Default|GetHealth) harm)))
  (CallFunction|UpdataUI)
  (if (<= _output_get 0.0)
    (Variables|Default|Setisdead true)
    (Components|Movement|StopMovementImmediately (Variables|Character|GetCharacterMovement))
    (Utilities|FlowControl|Delay 3.0)
    (Actor|DestroyActor)))

(fn ConstructionScript
  (Variables|Default|SetHealth (Variables|Default|GetMaxHealth))
  (Variables|Default|SetAIControllerClass self "/Game/TPS_File/AI/AI_Controllor.AI_Controllor_C"))

(fn UpdataUI
  (bind _asai_ui (Utilities|Casting|CastToAI_UI (UserInterface|GetUserWidgetObject (Variables|Default|GetWidget))))
  (bind _output_get (Variables|Default|SetAs%20AI%20UI _asai_ui))
  (Progress|SetPercent (Variables|/Game/TPS_File/UI/AI_UI.AI_UI_C|Get血量 _output_get) (/ (Variables|Default|GetHealth) (Variables|Default|GetMaxHealth))))

(fn AIShoot)